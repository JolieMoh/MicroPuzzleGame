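; Turbo lift actor that carries the first-person player between two relative positions and has a keypad-opened cabin door.
; A cylinder overlap while IsLocked is true waits briefly, then alternately plays or reverses the platform's lerp timeline, with a steam sound.
; Every BP_Keypad's OpenDoor event is bound to Open, which rotates the glass door.
; The door timeline clears IsLocked when opened and sets it when CloseDoor reverses it.
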(event OnComponentBeginOverlap(Cylinder)
  (params (OverlappedComponent :type Primitive%20Component%20Object%20Reference) (OtherActor :type Actor%20Object%20Reference) (OtherComp :type Primitive%20Component%20Object%20Reference) (OtherBodyIndex :type Integer) (bFromSweep :type Boolean) (SweepResult :type Hit%20Result%20Structure%20%28by%20ref%29))
  ;[1 1 1] Lift Motion
  (if (Variables|Default|GetIsLocked)
    (Utilities|Casting|CastToBP_FirstPersonCharacter OtherActor)
    (Utilities|FlowControl|Delay 0.8)
    (Utilities|FlowControl|FlipFlop
      (:A
        (Audio|Components|Audio|FadeIn (Variables|Default|GetSteam01_Cue) 0.1 1.0 0.0 "Linear" :!class /Script/Engine.AudioComponent)
        (bind _alpha (Timeline|Timeline Play)
          (:Update
            (Transformation|SetRelativeLocation (Variables|Default|GetSM_TurboLiftPlatform) (Math|Vector|Lerp(Vector) (.location (Variables|Default|GetStartRelative%20Location)) (.location (Variables|Default|GetEndtRelative%20Location_0)) _alpha) false false)
            (Audio|Components|Audio|FadeOut (Variables|Default|GetSteam01_Cue) 0.1 0.0 "Linear" :!class /Script/Engine.AudioComponent))))
      (:B
        (Audio|Components|Audio|FadeIn (Variables|Default|GetSteam01_Cue) 0.1 1.0 0.0 "Linear" :!class /Script/Engine.AudioComponent)
        (Timeline|Timeline Reverse)))))

(event Custom|Open
  ;[1 1 1] Unlocking Lift Door
  (bind (_direction _alpha) (Timeline|OpenDoor PlayFromStart)
    (:Update
      (Transformation|SetRelativeRotation (Variables|Default|GetSM_TurboLiftCabinGlass2) (Math|Rotator|Lerp(Rotator) "0, 0, 0" (Math|Rotator|MakeRotator 0.0 0.0 _alpha) 0.0) false false))
    (:Finished
      (switch Utilities|FlowControl|Switch|SwitchonETimelineDirection _direction
        (:Forward
          (Variables|Default|SetIsLocked false))
        (:Backward
          (Variables|Default|SetIsLocked true))))))

(event Custom|CloseDoor
  ;[1 1 1] Unlocking Lift Door
  (bind (_direction _alpha) (Timeline|OpenDoor Reverse)
    (:Update
      (Transformation|SetRelativeRotation (Variables|Default|GetSM_TurboLiftCabinGlass2) (Math|Rotator|Lerp(Rotator) "0, 0, 0" (Math|Rotator|MakeRotator 0.0 0.0 _alpha) 0.0) false false))
    (:Finished
      (switch Utilities|FlowControl|Switch|SwitchonETimelineDirection _direction
        (:Forward
          (Variables|Default|SetIsLocked false))
        (:Backward
          (Variables|Default|SetIsLocked true))))))

(event EventBeginPlay
  (Components|Timeline|SetPlayRate (Variables|Default|GetTimeline) 2.0)
  ;[1 1 1] Unlocking Lift Door
  (bind _outactors (Actor|GetAllActorsOfClass "/Game/BP/BP_Keypad.BP_Keypad_C"))
  (for _array_element _outactors
    (EventDispatchers|BindEventtoOpenDoor _array_element (delegate Custom|Open))))

(fn ConstructionScript)
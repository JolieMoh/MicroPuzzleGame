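; BP_Doors is a sliding double corridor door that opens automatically for the first-person character.
; Entering the DoorTrigger volume fades in the open sound and plays a Timeline, and leaving fades in the close sound and reverses it.
; The Timeline's Alpha lerps both door meshes' relative locations between start and end positions taken from marker components.
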(event OnComponentBeginOverlap(DoorTrigger)
  (params (OverlappedComponent :type Primitive%20Component%20Object%20Reference) (OtherActor :type Actor%20Object%20Reference) (OtherComp :type Primitive%20Component%20Object%20Reference) (OtherBodyIndex :type Integer) (bFromSweep :type Boolean) (SweepResult :type Hit%20Result%20Structure%20%28by%20ref%29))
  (Utilities|Casting|CastToBP_FirstPersonCharacter OtherActor)
  (Audio|Components|Audio|FadeIn (Variables|Default|GetDoorOpen_Cue) 0.1 1.0 0.0 "Linear" :!class /Script/Engine.AudioComponent)
  (bind _alpha (Timeline|Timeline Play)
    (:Update
      (Transformation|SetRelativeLocation (Variables|Default|GetSM_CoridorDoorLeft) (Math|Vector|Lerp(Vector) (.location (Variables|Default|GetLeftDoorStartPos)) (.location (Variables|Default|GetLeftDoorEndPos)) _alpha) false false)
      (Transformation|SetRelativeLocation (Variables|Default|GetSM_CoridorDoorRight) (Math|Vector|Lerp(Vector) (.location (Variables|Default|GetRightDoorStartPos)) (.location (Variables|Default|GetRightDoorEndPos)) _alpha) false false))))

(event OnComponentEndOverlap(DoorTrigger)
  (params (OverlappedComponent :type Primitive%20Component%20Object%20Reference) (OtherActor :type Actor%20Object%20Reference) (OtherComp :type Primitive%20Component%20Object%20Reference) (OtherBodyIndex :type Integer))
  (Utilities|Casting|CastToBP_FirstPersonCharacter OtherActor)
  (Audio|Components|Audio|FadeIn (Variables|Default|GetDoorClose_Cue) 0.1 1.0 0.0 "Linear" :!class /Script/Engine.AudioComponent)
  (bind _alpha (Timeline|Timeline Reverse)
    (:Update
      (Transformation|SetRelativeLocation (Variables|Default|GetSM_CoridorDoorLeft) (Math|Vector|Lerp(Vector) (.location (Variables|Default|GetLeftDoorStartPos)) (.location (Variables|Default|GetLeftDoorEndPos)) _alpha) false false)
      (Transformation|SetRelativeLocation (Variables|Default|GetSM_CoridorDoorRight) (Math|Vector|Lerp(Vector) (.location (Variables|Default|GetRightDoorStartPos)) (.location (Variables|Default|GetRightDoorEndPos)) _alpha) false false))))

(fn ConstructionScript)
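; BP_RoomDoor is an interactable room door that swings open and closed.
; Each StartInteraction call alternates between OpenDoor and CloseDoor through a FlipFlop.
; The DoorSwing timeline plays forward to open and reverses to close, lerping the Door's relative rotation between DoorStartRotation and DoorEndRotation.
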(event Custom|OpenDoor
  (bind _alpha (Timeline|DoorSwing Play)
    (:Update
      (Transformation|SetRelativeRotation (Variables|Default|Getdoor) (Math|Rotator|Lerp(Rotator) (.rotation (Variables|Default|GetDoorStartRotation)) (.rotation (Variables|Default|GetDoorEndRotation)) _alpha) false false))))

(event Custom|CloseDoor
  (bind _alpha (Timeline|DoorSwing Reverse)
    (:Update
      (Transformation|SetRelativeRotation (Variables|Default|Getdoor) (Math|Rotator|Lerp(Rotator) (.rotation (Variables|Default|GetDoorStartRotation)) (.rotation (Variables|Default|GetDoorEndRotation)) _alpha) false false))))

(event EventStartInteraction
  (Utilities|FlowControl|FlipFlop
    (:A
      (CallFunction|OpenDoor))
    (:B
      (CallFunction|CloseDoor))))

(fn ConstructionScript)
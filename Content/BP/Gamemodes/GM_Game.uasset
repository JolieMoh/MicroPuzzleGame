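; GM_Game is the game mode that scatters engine pickups at match start and handles the end-game check.
; On BeginPlay, SpawnItems picks random BP_SpawnPoint actors, spawns BP_PickupEngine there, and removes each used point to avoid duplicate locations.
; TaskCompletion checks that the engine stand and wires tasks are complete and the turbo lift is moving, then shows W_GameOver with UI-only input and a visible cursor.
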(event EventBeginPlay
  (CallFunction|SpawnItems))

(fn ConstructionScript)

(fn SpawnItems
  (bind _outactors (Actor|GetAllActorsOfClass "/Game/BP/BP_SpawnPoint.BP_SpawnPoint_C"))
  (LocalVariables|SetLocalSpawnReferences _outactors)
  ;[1 1 1] 8 Pickups Needed
  (for _index (range 1 (Variables|Default|GetMaxNumOfItemsNeeded))
    (LocalVariables|SetLocalItem (.OutItem (Utilities|Array|Random (LocalVariables|GetLocalSpawnReferences))))
    (Game|SpawnActorfromClass "/Game/BP/BP_PickupEngine.BP_PickupEngine_C" (Math|Transform|MakeTransform (Transformation|GetActorLocation (LocalVariables|GetLocalItem)) "0.000000,0.000000,90.000000") "AdjustIfPossibleButAlwaysSpawn" "MultiplyWithRoot" 0 0)
    ;[1 1 1] Make sure the actors dont spawn at the same location
    (Utilities|Array|RemoveItem (LocalVariables|GetLocalSpawnReferences) (LocalVariables|GetLocalItem))
    (Actor|DestroyActor (LocalVariables|GetLocalItem))))

(fn TaskCompletion
  (bind _returnvalue (Game|GetPlayerController 0))
  (bind _returnvalue_2 (Actor|GetActorOfClass "/Game/BP/BP_EngineMainLarge_Stand.BP_EngineMainLarge_Stand_C"))
  (if (Variables|/Game/BP/BP_EngineMainLarge_Stand.BP_EngineMainLarge_Stand_C|GetIsTaskCompleted _returnvalue_2)
    (bind _returnvalue_3 (Actor|GetActorOfClass "/Game/BP/BP_Wires.BP_Wires_C"))
    (if (Variables|/Game/BP/BP_Wires.BP_Wires_C|GetIsTaskCompleted _returnvalue_3)
      (bind _returnvalue_4 (Actor|GetActorOfClass "/Game/BP/BP_TurboLift.BP_TurboLift_C"))
      (if (Variables|/Game/BP/BP_TurboLift.BP_TurboLift_C|GetIsLiftMoving _returnvalue_4)
        ;[1 1 1] Call End Game
        (bind _returnvalue_5 (UserInterface|CreateWidget "/Game/Widget/W_GameOver.W_GameOver_C"))
        (UserInterface|Viewport|AddtoViewport _returnvalue_5 0)
        (Input|SetInputModeUIOnly _returnvalue 0 "DoNotLock" false)
        (Variables|/Script/Engine.PlayerController|SetbShowMouseCursor _returnvalue true)))))
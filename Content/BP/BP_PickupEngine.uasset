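; Engine part pickup that the first-person character carries, drops or installs on the large engine stand.
; Interaction attaches it to the character's holding position, one part at a time; putting down restores physics and applies an impulse built from camera location plus scaled forward vector.
; StartLerping makes Tick interpolate it onto a preview reference, then it snaps, spawns brief sparks, destroys the preview and notifies the engine.
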(event Custom|PutDown
  (bind _staticmesh (Variables|Default|GetStaticMesh))
  (bind _fpcharacter (Variables|Default|GetFPCharacter))
  ;[1 1 1] Put Down
  (CallFunction|EnablePhysics)
  (Collision|SetCollisionEnabled (Variables|Default|GetStaticMesh) "QueryAndPhysics")
  (Transformation|DetachFromActor "KeepWorld" "KeepWorld" "KeepWorld")
  (CallFunction|LaunchDropObject)
  (Audio|PlaySoundatLocation "/Engine/VREditor/Sounds/UI/Drop_Item_From_ContentBrowser.Drop_Item_From_ContentBrowser" (Transformation|GetWorldLocation _staticmesh) (Transformation|GetWorldRotation _staticmesh) 1.0 1.0 0.0 "/Game/AbsoluteSpaceAndSciFi_VoltzSupreme/NewSoundAttenuation.NewSoundAttenuation" 0 0 0)
  (Variables|/Game/FirstPerson/Blueprints/BP_FirstPersonCharacter.BP_FirstPersonCharacter_C|SetIsHoldingEnginePart _fpcharacter false)
  (Variables|/Game/FirstPerson/Blueprints/BP_FirstPersonCharacter.BP_FirstPersonCharacter_C|SetCurrentEnginePartPickUp _fpcharacter 0))

(event Custom|StopLerping
  (bind _fpcharacter (Variables|Default|GetFPCharacter))
  ;[1 1 1] Setting Collision and Gravity when Lerping
  (Collision|SetCollisionEnabled (Variables|Default|GetStaticMesh) "QueryAndPhysics")
  (Variables|Default|SetShouldLerp? false)
  (Variables|/Game/FirstPerson/Blueprints/BP_FirstPersonCharacter.BP_FirstPersonCharacter_C|SetIsHoldingEnginePart _fpcharacter false)
  (Variables|/Game/FirstPerson/Blueprints/BP_FirstPersonCharacter.BP_FirstPersonCharacter_C|SetCurrentEnginePartPickUp _fpcharacter 0))

(event Custom|StartLerping
  (params (PreviewReference :type BP%20Engine%20Part%20Preview%20Object%20Reference))
  (bind _staticmesh (Variables|Default|GetStaticMesh))
  ;[1 1 1] Setting Collision and Gravity when Lerping
  (Variables|Default|SetPreview%20Reference PreviewReference)
  (Transformation|DetachFromComponent (Variables|Default|GetStaticMesh) "KeepWorld" "KeepWorld" "KeepWorld" true)
  (Collision|SetCollisionEnabled _staticmesh "NoCollision")
  (Physics|SetEnableGravity _staticmesh false)
  (CallFunction|DisablePhysics)
  (Variables|Default|SetShouldLerp? true)
  (Audio|PlaySoundatLocation "/Game/UI_SFX_Free_Pack/Wavs/Repair/repair_100.repair_100" (Transformation|GetActorLocation (Variables|Default|GetPreview%20Reference)) "0, 0, 0" 1.0 1.0 0.0 "/Game/AbsoluteSpaceAndSciFi_VoltzSupreme/NewSoundAttenuation.NewSoundAttenuation" 0 0 0))

(event EventTick
  (params (DeltaSeconds :type Float%20%28single-precision%29))
  (bind _returnvalue (Transformation|GetActorLocation))
  (bind _preview_reference (Variables|Default|GetPreview%20Reference))
  (bind _preview_reference_2 (Variables|Default|GetPreview%20Reference))
  (bind _returnvalue_2 (Transformation|GetActorLocation _preview_reference))
  (bind _returnvalue_3 (Transformation|GetActorTransform _preview_reference_2))
  ;[1 1 1] Lerp Current Pickup to Preview Mesh
  (if (Variables|Default|GetShouldLerp?)
    (Transformation|SetActorLocationAndRotation (Math|Interpolation|VInterpTo _returnvalue _returnvalue_2 DeltaSeconds 5.0) (Math|Interpolation|RInterpTo (Transformation|GetActorRotation) (Transformation|GetActorRotation (Variables|Default|GetPreview%20Reference)) DeltaSeconds 5.0))
    (if (< (Math|Vector|Distance(Vector) _returnvalue _returnvalue_2) 0.1)
      (Transformation|SetActorTransform _returnvalue_3 false true)
      (CallFunction|StopLerping)
      (bind _returnvalue_4 (Game|SpawnActorfromClass "/Game/StarterContent/Blueprints/Blueprint_Effect_Sparks.Blueprint_Effect_Sparks_C" _returnvalue_3 "Undefined" "MultiplyWithRoot" 0 0))
      (Utilities|FlowControl|Delay 0.3)
      (Actor|DestroyActor _returnvalue_4)
      (Default|PieceInstalled (Variables|Default|GetEngine)))))

(event EventBeginPlay
  (bind _returnvalue (Actor|GetActorOfClass "/Game/BP/BP_EngineMainLarge_Stand.BP_EngineMainLarge_Stand_C"))
  (Variables|Default|SetEngine _returnvalue)
  (bind _returnvalue_2 (Actor|GetActorOfClass "/Game/FirstPerson/Blueprints/BP_FirstPersonCharacter.BP_FirstPersonCharacter_C"))
  (Variables|Default|SetFPCharacter _returnvalue_2))

(event EventStartInteraction
  (bind _fpcharacter (Variables|Default|GetFPCharacter))
  ;[1 1 1] Pick UP
  (if (not (Variables|/Game/FirstPerson/Blueprints/BP_FirstPersonCharacter.BP_FirstPersonCharacter_C|GetIsHoldingEnginePart (Variables|Default|GetFPCharacter)))
    (Variables|/Game/FirstPerson/Blueprints/BP_FirstPersonCharacter.BP_FirstPersonCharacter_C|SetIsHoldingEnginePart _fpcharacter true)
    (Variables|/Game/FirstPerson/Blueprints/BP_FirstPersonCharacter.BP_FirstPersonCharacter_C|SetCurrentEnginePartPickUp _fpcharacter self)
    (CallFunction|DisablePhysics)
    (Collision|SetCollisionEnabled (Variables|Default|GetStaticMesh) "NoCollision")
    (Transformation|AttachComponentToComponent (Variables|/Game/FirstPerson/Blueprints/BP_FirstPersonCharacter.BP_FirstPersonCharacter_C|GetHoldingPosition (Variables|Default|GetFPCharacter)) "None" "SnapToTarget" "SnapToTarget" "KeepRelative" true)
    (Audio|PlaySound2D "/Engine/VREditor/Sounds/UI/Object_PickUp.Object_PickUp" 1.0 1.0 0.0 0 0)))

(fn ConstructionScript)

(fn DisablePhysics
  (Physics|SetSimulatePhysics (Variables|Default|GetStaticMesh) false))

(fn EnablePhysics
  (Physics|SetSimulatePhysics (Variables|Default|GetStaticMesh) true))

(fn LaunchDropObject
  (bind _fpcharacter (Variables|Default|GetFPCharacter))
  (bind _firstpersoncamera (Variables|/Game/FirstPerson/Blueprints/BP_FirstPersonCharacter.BP_FirstPersonCharacter_C|GetFirstPersonCamera _fpcharacter))
  (Physics|AddImpulse (Variables|Default|GetStaticMesh) (+ (Transformation|GetWorldLocation _firstpersoncamera) (* (Math|Vector|GetForwardVector _firstpersoncamera) (Variables|Default|GetLaunchMultiplier))) "None" false)
  (return))
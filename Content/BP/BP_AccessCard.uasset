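; Access card actor that snaps to a card reader and animates a swipe through it.
; StartLerping plays a snap sound, disables collision and gravity, and lets Tick interpolate the mesh toward the start transform of the BP_CardReader found at BeginPlay.
; On arrival it restores collision and gravity, waits, then runs a Timeline between the reader's start and end transforms.
; Separate functions toggle physics simulation on the mesh.
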(event Custom|StopLerping
  (bind _staticmesh (Variables|Default|GetStaticMesh))
  ;[1 1 1] Setting Collision and Gravity when Lerping
  (Collision|SetCollisionEnabled _staticmesh "QueryAndPhysics")
  (Physics|SetEnableGravity _staticmesh true)
  (Variables|Default|SetShouldLerp? false))

(event Custom|StartLerping
  (bind _staticmesh (Variables|Default|GetStaticMesh))
  ;[1 1 1] Setting Collision and Gravity when Lerping
  (Collision|SetCollisionEnabled _staticmesh "NoCollision")
  (Physics|SetEnableGravity _staticmesh false)
  (Variables|Default|SetShouldLerp? true)
  (Audio|PlaySoundatLocation "/Engine/VREditor/Sounds/UI/Object_Snaps_To_Another_Actor.Object_Snaps_To_Another_Actor" (Transformation|GetActorLocation (Variables|Default|GetCardReader)) "0, 0, 0" 1.0 1.0 0.0 "/Game/AbsoluteSpaceAndSciFi_VoltzSupreme/NewSoundAttenuation.NewSoundAttenuation" 0 0 0))

(event Custom|SwipeCard
  (bind _cardreader (Variables|Default|GetCardReader))
  (bind _cardendposition (Variables|/Game/BP/BP_CardReader.BP_CardReader_C|GetCardEndPosition _cardreader))
  (bind _cardstartposition (Variables|/Game/BP/BP_CardReader.BP_CardReader_C|GetCardStartPosition _cardreader))
  ;[1 1 1] Swipe Card Animation
  (bind _alpha (Timeline|Timeline Play)
    (:Update
      (Transformation|SetRelativeLocationAndRotation (Variables|Default|GetStaticMesh) (Math|Vector|Lerp(Vector) (.location _cardstartposition) (.location _cardendposition) _alpha) (Math|Rotator|Lerp(Rotator) (.rotation _cardstartposition) (.rotation _cardendposition) _alpha) false false)
      (if (< (Math|Vector|Distance(Vector) (.location _cardstartposition) (.location _cardendposition)) 0.1)
        (Transformation|SetRelativeTransform (Variables|Default|GetStaticMesh) (Variables|/Game/BP/BP_CardReader.BP_CardReader_C|GetCardEndPosition (Variables|Default|GetCardReader)) false false)))))

(event EventTick
  (params (DeltaSeconds :type Float%20%28single-precision%29))
  (bind _returnvalue (Transformation|GetActorLocation))
  (bind _cardreader (Variables|Default|GetCardReader))
  (bind _cardstartposition (Variables|/Game/BP/BP_CardReader.BP_CardReader_C|GetCardStartPosition _cardreader))
  ;[1 1 1] Lerp Card to Reader
  (if (Variables|Default|GetShouldLerp?)
    (Transformation|SetRelativeLocationAndRotation (Variables|Default|GetStaticMesh) (Math|Interpolation|VInterpTo _returnvalue (.location _cardstartposition) DeltaSeconds 5.0) (Math|Interpolation|RInterpTo (Transformation|GetActorRotation) (.rotation _cardstartposition) DeltaSeconds 5.0) false false)
    (if (< (Math|Vector|Distance(Vector) _returnvalue (.location _cardstartposition)) 0.1)
      (Transformation|SetRelativeTransform (Variables|Default|GetStaticMesh) (Variables|/Game/BP/BP_CardReader.BP_CardReader_C|GetCardStartPosition (Variables|Default|GetCardReader)) false false)
      (CallFunction|StopLerping)
      (Utilities|FlowControl|Delay 5.0)
      (CallFunction|SwipeCard))))

(event EventBeginPlay
  (bind _returnvalue (Actor|GetActorOfClass "/Game/BP/BP_CardReader.BP_CardReader_C"))
  (Variables|Default|SetCardReader _returnvalue))

(fn ConstructionScript)

(fn DisablePhysics
  (Physics|SetSimulatePhysics (Variables|Default|GetStaticMesh) false))

(fn EnablePhysics
  (Physics|SetSimulatePhysics (Variables|Default|GetStaticMesh) true))
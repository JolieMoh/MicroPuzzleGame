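; Interactable keypad that unlocks a door when the entered combination matches its passcode.
; StartInteraction shows the cursor, switches to UI-only input and opens a W_Keypad widget that holds a reference back to the keypad.
; TriggerDoor checks the combination, fires the OpenDoor dispatcher on a match and swaps the mesh's keypad and light materials to show unlocked green or locked red.
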(event Custom|TriggerDoor
  (params (Combo :type String))
  (bind _staticmesh (Variables|Default|GetStaticMesh))
  (bind _staticmesh_2 (Variables|Default|GetStaticMesh))
  (if (Utilities|Enum|Equal(Enum) Combo (Variables|Default|GetPassCode))
    (Default|CallOpenDoor)
    (Rendering|Material|SetMaterial _staticmesh 0 "/Game/StarterBundle/ModularScifiProps/Materials/MI_Keypad_Unlocked.MI_Keypad_Unlocked")
    (Rendering|Material|SetMaterial _staticmesh 2 "/Game/StarterBundle/ModularScifiProps/Materials/MI_Light_Green.MI_Light_Green")
    (else
      (Rendering|Material|SetMaterial _staticmesh_2 0 "/Game/StarterBundle/ModularScifiProps/Materials/MI_Keypad_Locked.MI_Keypad_Locked")
      (Rendering|Material|SetMaterial _staticmesh_2 2 "/Game/StarterBundle/ModularScifiProps/Materials/MI_Light_Red.MI_Light_Red"))))

(event EventStartInteraction
  (bind _returnvalue (Game|GetPlayerController 0))
  (Variables|/Script/Engine.PlayerController|SetbShowMouseCursor _returnvalue true)
  (Input|SetInputModeUIOnly _returnvalue 0 "DoNotLock" false)
  (bind _returnvalue_2 (UserInterface|CreateWidget "/Game/Widget/W_Keypad.W_Keypad_C" 0 self))
  (UserInterface|Viewport|AddtoViewport _returnvalue_2 0))

(fn ConstructionScript)
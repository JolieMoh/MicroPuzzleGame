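; BP_Wires is a wire-connection puzzle built from four child BP_Wire actors.
; The construction script collects the wires, colors each from a color array and shuffles their attach locations among them.
; An attach handler plays a sound once IsCompleted finds all wires successful, but its binding is disconnected, leaving the BeginPlay loop empty.
; StartInteraction is a stub, and IsCompleted appends to its results list without clearing it.
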(event Custom|OnAttached_Event
  (if (CallFunction|IsCompleted)
    (Audio|PlaySoundatLocation "/Engine/EditorSounds/GamePreview/StartSimulate_Cue.StartSimulate_Cue" (Transformation|GetWorldLocation (Variables|Default|GetScene)) "0, 0, 0" 1.0 1.0 0.0 "/Game/AbsoluteSpaceAndSciFi_VoltzSupreme/NewSoundAttenuation.NewSoundAttenuation" 0 0 0)))

(event EventBeginPlay
  (for _array_element (Variables|Default|GetWires)
    _))

(event EventStartInteraction)

(fn ConstructionScript
  (Utilities|FlowControl|Sequence
    (:then_0
      (for _array_element (Utilities|Array|MakeArray (Variables|Default|GetChildActor1) (Variables|Default|GetChildActor2) (Variables|Default|GetChildActor3) (Variables|Default|GetChildActor))
        (bind _asbp_wire (Utilities|Casting|CastToBP_Wire (Variables|/Script/Engine.ChildActorComponent|GetChildActor _array_element)))
        (Utilities|Array|Add (Variables|Default|GetWires) _asbp_wire)))
    (:then_1
      (for (_array_element_2 _array_index) (Variables|Default|GetWires)
        (Default|SetWireColor _array_element_2 (Utilities|Array|Get(acopy) (Variables|Default|GetColors) _array_index))))
    (:then_2
      (CallFunction|ShuffleEndLocation))))

(fn ShuffleEndLocation
  (Utilities|FlowControl|Sequence
    (:then_0
      (for _array_element (Variables|Default|GetWires)
        (Utilities|Array|Add (Variables|Default|GetLocation_L) (Default|GetAttachLocation _array_element))))
    (:then_1
      (Utilities|Array|Shuffle (Variables|Default|GetLocation_L)))
    (:then_2
      (for (_array_element_2 _array_index) (Variables|Default|GetWires)
        (Default|SetAttachLocation _array_element_2 (Utilities|Array|Get(acopy) (Variables|Default|GetLocation_L) _array_index))))))

(fn IsCompleted
  (for _array_element (Variables|Default|GetWires)
    (Utilities|Array|Add (Variables|Default|GetIs%20Successful_L) (Variables|/Game/BP/BP_Wire.BP_Wire_C|GetIsSuccessful _array_element)))
  (return (not (Utilities|Array|ContainsItem (Variables|Default|GetIs%20Successful_L) false))))
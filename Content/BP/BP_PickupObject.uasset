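; Pickup actor for an engine piece that installs onto the BP_EngineMainLarge_Stand found at BeginPlay.
; A trigger shows its widget while the first-person character overlaps, and events toggle mesh physics simulation.
; StartLerping disables collision and gravity, plays a repair sound, and Tick interpolates the actor toward a preview actor.
; On arrival it snaps into place, restores collision and gravity, destroys the preview and calls PieceInstalled on the engine.
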(event OnComponentBeginOverlap(Trigger)
  (params (OverlappedComponent :type Primitive%20Component%20Object%20Reference) (OtherActor :type Actor%20Object%20Reference) (OtherComp :type Primitive%20Component%20Object%20Reference) (OtherBodyIndex :type Integer) (bFromSweep :type Boolean) (SweepResult :type Hit%20Result%20Structure%20%28by%20ref%29))
  ;[1 1 1] Widget Visibility
  (Utilities|Casting|CastToBP_FirstPersonCharacter OtherActor)
  (Rendering|SetVisibility (Variables|Default|GetWidget) true false))

(event OnComponentEndOverlap(Trigger)
  (params (OverlappedComponent :type Primitive%20Component%20Object%20Reference) (OtherActor :type Actor%20Object%20Reference) (OtherComp :type Primitive%20Component%20Object%20Reference) (OtherBodyIndex :type Integer))
  ;[1 1 1] Widget Visibility
  (Utilities|Casting|CastToBP_FirstPersonCharacter OtherActor)
  (Rendering|SetVisibility (Variables|Default|GetWidget) false false))

(event Custom|EnablePhysics
  ;[1 1 1] Call Enable/Disable Physics
  (Physics|SetSimulatePhysics (Variables|Default|GetStaticMesh) true))

(event Custom|DisablePhysics
  ;[1 1 1] Call Enable/Disable Physics
  (Physics|SetSimulatePhysics (Variables|Default|GetStaticMesh) false))

(event Custom|StopLerping
  (bind _staticmesh (Variables|Default|GetStaticMesh))
  ;[1 1 1] Setting Collision and Gravity when Lerping
  (Collision|SetCollisionEnabled _staticmesh "QueryAndPhysics")
  (Physics|SetEnableGravity _staticmesh true)
  (Collision|SetCollisionEnabled (Variables|Default|GetTrigger) "QueryAndPhysics")
  (Variables|Default|SetShouldLerp? false))

(event Custom|StartLerping
  (params (PreviewReference :type Actor%20Object%20Reference))
  (bind _staticmesh (Variables|Default|GetStaticMesh))
  ;[1 1 1] Setting Collision and Gravity when Lerping
  (Variables|Default|SetPreview%20Reference PreviewReference)
  (Collision|SetCollisionEnabled _staticmesh "NoCollision")
  (Physics|SetEnableGravity _staticmesh false)
  (Collision|SetCollisionEnabled (Variables|Default|GetTrigger) "NoCollision")
  (Variables|Default|SetShouldLerp? true)
  (Audio|PlaySoundatLocation "/Game/UI_SFX_Free_Pack/Wavs/Repair/repair_100.repair_100" (Transformation|GetActorLocation) "0, 0, 0" 1.0 1.0 0.0 0 0 0 0))

(event EventTick
  (params (DeltaSeconds :type Float%20%28single-precision%29))
  (bind _returnvalue (Transformation|GetActorLocation))
  (bind _preview_reference (Variables|Default|GetPreview%20Reference))
  (bind _returnvalue_2 (Transformation|GetActorLocation _preview_reference))
  ;[1 1 1] Lerp Current Pickup to Preview Mesh
  (if (Variables|Default|GetShouldLerp?)
    (Transformation|SetActorLocationAndRotation (Math|Interpolation|VInterpTo _returnvalue _returnvalue_2 DeltaSeconds 5.0) (Math|Interpolation|RInterpTo (Transformation|GetActorRotation) (Transformation|GetActorRotation (Variables|Default|GetPreview%20Reference)) DeltaSeconds 5.0))
    (if (< (Math|Vector|Distance(Vector) _returnvalue _returnvalue_2) 0.1)
      (Transformation|SetActorTransform (Transformation|GetActorTransform (Variables|Default|GetPreview%20Reference)) false true)
      (CallFunction|StopLerping)
      (Actor|DestroyActor (Variables|Default|GetPreview%20Reference))
      (Default|PieceInstalled (Variables|Default|GetEngine)))))

(event EventBeginPlay
  (bind _returnvalue (Actor|GetActorOfClass "/Game/BP/BP_EngineMainLarge_Stand.BP_EngineMainLarge_Stand_C"))
  (Variables|Default|SetEngine _returnvalue))

(fn ConstructionScript)
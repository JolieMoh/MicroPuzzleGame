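; BP_EnginePart_Preview is a transparent placeholder for an engine part that serves as a target for the part the player picks up.
; The construction script and BeginPlay apply MeshToUse, falling back to Engine_Shell_1, and BeginPlay also sets the transparent material.
; StartInteraction calls StartLerping on the first-person character's CurrentEnginePartPickUp, if valid, passing this preview as the target.
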(event EventBeginPlay
  (bind _enginepart (Variables|Default|GetEnginePart))
  (bind _returnvalue (Actor|GetActorOfClass "/Game/FirstPerson/Blueprints/BP_FirstPersonCharacter.BP_FirstPersonCharacter_C"))
  (Variables|Default|SetFPCharacter _returnvalue)
  (bind _returnvalue_2 (Actor|GetActorOfClass "/Game/BP/BP_PickupEngine.BP_PickupEngine_C"))
  (Variables|Default|SetPickUpEnginePart _returnvalue_2)
  ;[1 1 1] Override Mat to Transparent Material
  (Rendering|Material|SetMaterial (Variables|Default|GetEnginePart) 0 "/Game/CSDefender/Materials/MI_EngineMainLarge_Transparent.MI_EngineMainLarge_Transparent")
  ;[1 1 1] Check if mesh is valid
  (if (Utilities|IsValid (Variables|Default|GetMeshToUse))
    (Components|StaticMesh|SetStaticMesh _enginepart (Variables|Default|GetMeshToUse))
    (else
      (bind _output_get (Variables|Default|SetMeshToUse "/Game/CSDefender/Mesh/Machines/EngineLargeParts/Engine_Shell_1.Engine_Shell_1"))
      (Components|StaticMesh|SetStaticMesh _enginepart _output_get))))

(event EventStartInteraction
  (if (Utilities|IsValid (Variables|/Game/FirstPerson/Blueprints/BP_FirstPersonCharacter.BP_FirstPersonCharacter_C|GetCurrentEnginePartPickUp (Variables|Default|GetFPCharacter)))
    (Default|StartLerping (Variables|/Game/FirstPerson/Blueprints/BP_FirstPersonCharacter.BP_FirstPersonCharacter_C|GetCurrentEnginePartPickUp (Variables|Default|GetFPCharacter)) self)))

(fn ConstructionScript
  (bind _enginepart (Variables|Default|GetEnginePart))
  ;[1 1 1] Check if mesh is valid
  (if (Utilities|IsValid (Variables|Default|GetMeshToUse))
    (Components|StaticMesh|SetStaticMesh _enginepart (Variables|Default|GetMeshToUse))
    (else
      (bind _output_get (Variables|Default|SetMeshToUse "/Game/CSDefender/Mesh/Machines/EngineLargeParts/Engine_Shell_1.Engine_Shell_1"))
      (Components|StaticMesh|SetStaticMesh _enginepart _output_get))))
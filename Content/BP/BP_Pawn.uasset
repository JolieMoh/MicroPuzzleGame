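; Player pawn that lets the player drag BP_Wire actors with the left mouse button and connect them to other wires.
; On press, a cursor trace picks a grabbable wire component, and on release a second trace attaches it to a valid target wire or resets it.
; While held, Tick moves the wire's end to where the cursor ray intersects a plane through the wire, facing along its forward vector.
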(event Custom|EndGrab
  (bind _returnvalue (Game|GetPlayerController 0))
  (bind (_worldlocation _worlddirection) (Game|Player|ConvertMouseLocationToWorldSpace _returnvalue))
  ;[1 1 1] End Grab
  (Variables|Default|GetGrabWire
    (:then
      (bind (_outhit _returnvalue_2) (Collision|LineTraceByChannel _worldlocation (+ _worldlocation (* _worlddirection 1e+04)) "TraceTypeQuery1" false 0 "ForOneFrame"))
      (if _returnvalue_2
        (bind _asbp_wire (Utilities|Casting|CastToBP_Wire (.hitactor _outhit))
          (:then
            (if (Default|CanAttach _asbp_wire (.hitcomponent _outhit))
              (Default|Attach (Variables|Default|GetGrabWire) _asbp_wire)
              (Variables|Default|SetGrabWire 0)
              (else
                (CallFunction|ResetGrab))))
          (:CastFailed
            (CallFunction|ResetGrab)))
        (else
          (CallFunction|ResetGrab))))
    (:else)))

(event Custom|StartGrab
  (bind _returnvalue (Game|GetPlayerController 0))
  (bind (_worldlocation _worlddirection) (Game|Player|ConvertMouseLocationToWorldSpace _returnvalue))
  ;[1 1 1] Start Grab
  (bind (_outhit _returnvalue_2) (Collision|LineTraceByChannel _worldlocation (+ _worldlocation (* _worlddirection 1e+04)) "TraceTypeQuery1" false 0 "ForOneFrame"))
  (if _returnvalue_2
    (bind _asbp_wire (Utilities|Casting|CastToBP_Wire (.hitactor _outhit)))
    (if (Default|CanGrab _asbp_wire (.hitcomponent _outhit))
      (bind _output_get (Variables|Default|SetGrabWire _asbp_wire))
      (Default|StartGrab _output_get))
    (else
      (CallFunction|ResetGrab))))

(event Custom|UpdateGrab
  (bind _returnvalue (Game|GetPlayerController 0))
  (bind (_worldlocation _worlddirection) (Game|Player|ConvertMouseLocationToWorldSpace _returnvalue))
  ;[1 1 1] Update Grab location to mouse
  (bind _grabwire (Variables|Default|GetGrabWire)
    (:then
      (if (.ReturnValue (Class|KismetMathLibrary|LinePlaneIntersectionOriginNormal _worldlocation (+ _worldlocation (* _worlddirection 1e+04)) (Transformation|GetActorLocation _grabwire) (Transformation|GetActorForwardVector _grabwire)))
        (Default|SetEndLocation _grabwire (.Intersection (Class|KismetMathLibrary|LinePlaneIntersectionOriginNormal _worldlocation (+ _worldlocation (* _worlddirection 1e+04)) (Transformation|GetActorLocation _grabwire) (Transformation|GetActorForwardVector _grabwire))))))
    (:else)))

(event Custom|ResetGrab
  ;[1 1 1] Reset Wire Locations
  (bind _grabwire (Variables|Default|GetGrabWire)
    (:then
      (Default|Reset _grabwire)
      (Variables|Default|SetGrabWire 0))
    (:else)))

(event EventTick
  (params (DeltaSeconds :type Float%20%28single-precision%29))
  (CallFunction|UpdateGrab))

(event Input|MouseEvents|LeftMouseButton
  (params (Key :type Key%20Structure :default "None"))
  ;[1 1 1] LMB Control
  (:Pressed
    (CallFunction|StartGrab))
  (:Released
    (CallFunction|EndGrab)))

(fn ConstructionScript)